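; BP_TanukiPlayer is the player-controlled Tanuki, set up with what appears to be samurai duel input.
; On BeginPlay it runs the parent logic, has player controller 0 possess it, and adds the IMC_Duel_Samurai mapping context through Enhanced Input.
; The Tanuki attack input action prints a debug string and calls Attack, which is defined outside these graphs.
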(event Input|EnhancedActionEvents|EnhancedInputActionIA_Tankuki_Attack
  (params (ActionValue :type Boolean) (ElapsedSeconds :type Float%20%28double-precision%29) (TriggeredSeconds :type Float%20%28double-precision%29) (InputAction :type Input%20Action%20Object%20Reference :default "/Game/Input/Actions/IA_Tankuki_Attack.IA_Tankuki_Attack"))
  (:Started
    (Development|PrintString "Tanuki Attack")
    (CallFunction|Attack)))

(event EventBeginPlay
  (|CallParentFunction)
  (Pawn|Possess (Game|GetPlayerController 0) self)
  (bind _asplayer_controller (Utilities|Casting|CastToPlayerController (Pawn|GetController)))
  (Input|AddMappingContext (PlayerController|LocalPlayerSubsystems|GetEnhancedInputLocalPlayerSubsystem _asplayer_controller) "/Game/Input/IMC_Duel_Samurai.IMC_Duel_Samurai" 0 "(bIgnoreAllPressedKeysUntilRelease=True,bForceImmediately=False)"))

(fn ConstructionScript
  (|CallParentFunction))