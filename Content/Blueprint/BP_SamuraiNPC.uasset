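; BP_SamuraiNPC is the computer-controlled samurai that attacks during the game's draw phase.
; On BeginPlay it runs the parent logic and subscribes to the GameMode's draw-phase-started event.
; When that phase starts, it waits a random delay between its minimum and maximum NPC attack delay, then calls Attack, simulating a variable reaction time.
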(event Custom|OnDrawPhaseStarted
  (Utilities|FlowControl|Delay (Math|Random|RandomFloatinRange (Variables|Default|GetMinNPCAttackDelay) (Variables|Default|GetMaxNPCAttackDelay)))
  (CallFunction|Attack))

(event EventBeginPlay
  (|CallParentFunction)
  (EventDispatchers|BindEventtoDrawPhaseStarted (Variables|Default|GetGameMode) (delegate Custom|OnDrawPhaseStarted)))

(fn ConstructionScript
  (|CallParentFunction))