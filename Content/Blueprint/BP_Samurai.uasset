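; Sprite-based samurai duelist for the quick-draw duel run by GM_Duel, sliding into place at start and on Reset.
; Attack allows one press per round: during Wait it shows a cross and locks further input, during Draw it finishes the game.
; A winning press plays a fast timeline lunge that swaps to the attack sprite mid-motion and reports to GM_Duel whether the attacker is player-controlled.
; Defeated swaps to the defeat sprite and hides the cross.
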(event Custom|SlideIn
  (Components|Timeline|SetPlayRate (Variables|Default|GetSlideInAnim) 2.0)
  (bind _alpha (Timeline|SlideInAnim Play)
    (:Update
      (Transformation|SetRelativeLocation (Variables|Default|GetSamurai) (Math|Vector|Lerp(Vector) (Variables|Default|GetSlideStartPos) (Variables|Default|GetSprite%20Default) _alpha) false false))))

(event Custom|Attack
  (if (not (Variables|Default|GetPressedDraw))
    (switch Utilities|FlowControl|Switch|SwitchonE_Phase (Variables|/Game/Blueprint/GM_Duel.GM_Duel_C|GetPhase (Variables|Default|GetGameMode))
      (:NewEnumerator1
        (CallFunction|SetCrossVisibility true)
        (Variables|Default|SetPressedDraw true))
      (:NewEnumerator2
        (Variables|Default|SetPressedDraw true)
        (Default|SetGameFinished (Variables|Default|GetGameMode))
        (Components|Timeline|SetPlayRate (Variables|Default|GetAttackAnim) 8.0)
        (bind _alpha (Timeline|AttackAnim PlayFromStart)
          (:Update
            (Transformation|SetRelativeLocation (Variables|Default|GetSamurai) (Math|Vector|Lerp(Vector) (Variables|Default|GetSprite%20Default) (Variables|/Script/Engine.SceneComponent|GetRelativeLocation (Variables|Default|GetAttackPos)) _alpha) false false))
          (:SwitchSprite
            (CallFunction|SetSprite (Variables|Default|GetAttackSprite))
            (Default|AttackedSuccesfully (Variables|Default|GetGameMode) (Pawn|IsPlayerControlled))))))))

(event Custom|Defeated
  (Rendering|Components|Sprite|SetSprite (Variables|Default|GetSamurai) (Variables|Default|GetDefeatedSprite))
  (CallFunction|SetCrossVisibility false))

(event EventBeginPlay
  (bind _asgm_duel (Utilities|Casting|CastToGM_Duel (Game|GetGameMode)))
  (Variables|Default|SetGameMode _asgm_duel)
  (Variables|Default|SetRelative%20Location (Variables|/Script/Engine.SceneComponent|GetRelativeLocation (Variables|Default|GetSamurai)))
  (CallFunction|Slidein)
  (CallFunction|SetCrossVisibility false))

(fn ConstructionScript)

(fn SetCrossVisibility
  (params (bNewVisibility :type Boolean))
  (Rendering|SetVisibility (Variables|Default|GetCross) bNewVisibility false))

(fn SetSprite
  (params (NewSprite :type Paper%20Sprite%20Object%20Reference))
  (Rendering|Components|Sprite|SetSprite (Variables|Default|GetSamurai) NewSprite)
  (Rendering|Material|SetMaterial (Variables|Default|GetSamurai) 0 "/Paper2D/TranslucentUnlitSpriteMaterial.TranslucentUnlitSpriteMaterial")
  (Rendering|SetTranslucentSortPriority (Variables|Default|GetSamurai) 1))

(fn Reset
  (CallFunction|SetSprite (Variables|Default|GetIdleSprite))
  (Variables|Default|SetPressedDraw false)
  (CallFunction|Slidein))